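; Magnetic force component that pulls or pushes nearby objects, treating each owner's first actor tag as polarity: different tags attract, matching tags repel.
; Each tick, it scans Influence overlaps for eligible magnetic components, skipping "NoForce" owners, and applies opposite forces scaled by inverse distance to both objects.
; ApplyMagForce launches Characters with scaled-down velocity and pushes simulating physics bodies at their center of mass.
; Magnatized and ExternallyMagged flags track whether magnetism affects the object.
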(event `self.ReceiveTick`
  (params (DeltaSeconds :type "Float (single-precision)"))
  (bind _parent (`self.Parent`))
  (set `self.Magnatized` (`self.externally_magged`))
  (set `self.externally_magged` false)
  (if (or (`self.ApplyForce`) (!= (`|GetArrayItem` (`Actor.Tags` (`self.GetOwner` (`self.Parent`)))) "NoForce"))
    (for _array_element (`PrimitiveComponent.GetOverlappingComponents` (`self.Influence`))
      (if (!= _array_element _parent)
        (bind _returnvalue (`self.GetOwner` _array_element))
        (bind _output (`|GetArrayItem` (`Actor.Tags` _returnvalue)))
        (if (== _output "NoForce")
          _
          (elif (`/Game/Game/PlayerCharacter/Blueprints/MagneticForce.ApplyForce` (`Actor.GetComponentByClass` _returnvalue "MagneticForce_C"))
            (bind _returnvalue_2 (- (`PrimitiveComponent.GetCenterOfMass` _array_element "None") (`PrimitiveComponent.GetCenterOfMass` _parent "None")))
            (bind _returnvalue_3 (* (`KismetMathLibrary.Normal` _returnvalue_2) (* (* 10000000.0 (`KismetMathLibrary.SafeDivide` 1.0 (`KismetMathLibrary.VSize` _returnvalue_2))) (`KismetMathLibrary.SelectFloat` 1.0 -1.0 (!= (`|GetArrayItem` (`Actor.Tags` (`self.GetOwner` _parent))) _output)))))
            (`self.ApplyMagForce` (`self.Parent`) (* _returnvalue_3 0.5) DeltaSeconds)
            (set `self.Magnatized` true)
            (`self.ApplyMagForce` _array_element (* _returnvalue_3 -0.5))
            (set `/Game/Game/PlayerCharacter/Blueprints/MagneticForce.externally_magged` true (`Actor.GetComponentByClass` (`self.GetOwner` _array_element) "MagneticForce_C"))))))))

(fn `ApplyMagForce`
  (params (Object :type "PrimitiveComponent Object Reference") (Force :type "Vector Structure") (Delta :type "Float (double-precision)"))
  (bind _ascharacter (cast `Character` (`self.GetOwner` Object))
    (:`then`
      (`Character.LaunchCharacter` _ascharacter (* Force 0.001) false false))
    (:`CastFailed`
      (if (`SceneComponent.IsSimulatingPhysics` Object "None")
        (`PrimitiveComponent.AddForceAtLocation` Object Force (`PrimitiveComponent.GetCenterOfMass` Object "None") "None")))))