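; BadDude is a magnetic enemy character that moves toward and faces any player overlapping its sphere.
; Construction wires up its MagneticForce component and uses Positive or Negative actor tags to set polarity and matching fire effect.
; A hit from a dashing player knocks it away.
; After a short delay, if their polarities are opposite, it launches far harder, ragdolls, and disables magnetic force and capsule collision.
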(event `self.ReceiveTick`
  (params (DeltaSeconds :type "Float (single-precision)"))
  (bind _returnvalue (`PrimitiveComponent.GetCenterOfMass` (`self.ColSphere`) "None"))
  (for _array_element (`PrimitiveComponent.GetOverlappingComponents` (`self.ColSphere`))
    (bind _returnvalue_2 (`ActorComponent.GetOwner` _array_element))
    (if (!= _returnvalue_2 self)
      (if (== (`GameplayStatics.GetObjectClass` _returnvalue_2) "/Game/Game/PlayerCharacter/Blueprints/PLAYER_MainCharacter.PLAYER_MainCharacter_C")
        (bind _returnvalue_3 (`PrimitiveComponent.GetCenterOfMass` _array_element "None"))
        (`self.AddMovementInput` (* (`KismetMathLibrary.Normal` (- _returnvalue_3 _returnvalue)) 0.5))
        (`self.K2_SetActorRotation` (`KismetMathLibrary.FindLookAtRotation` (`KismetMathLibrary.MakeVector` (.x _returnvalue) (.y _returnvalue)) (`KismetMathLibrary.MakeVector` (.x _returnvalue_3) (.y _returnvalue_3))))))))

(event `self.ReceiveHit`
  (params (MyComp :type "PrimitiveComponent Object Reference") (Other :type "Actor Object Reference") (OtherComp :type "PrimitiveComponent Object Reference") (bSelfMoved :type Boolean) (HitLocation :type "Vector Structure") (HitNormal :type "Vector Structure") (NormalImpulse :type "Vector Structure") (Hit :type "HitResult Structure (by ref)"))
  (bind _returnvalue (`KismetMathLibrary.Normal` (- (`PrimitiveComponent.GetCenterOfMass` (`self.Mesh`) "None") (`PrimitiveComponent.GetCenterOfMass` (`Character.Mesh` (`self.Collider`)) "None"))))
  (bind _asplayer_main_character (cast `/Game/Game/PlayerCharacter/Blueprints/PLAYER_MainCharacter` Other))
  (bind _output_get (set `self.As PLAYER Main Character` _asplayer_main_character))
  (if (`/Game/Game/PlayerCharacter/Blueprints/PLAYER_MainCharacter.Is Dashing?` _output_get)
    (set `self.Collider` _asplayer_main_character)
    (`self.LaunchCharacter` (* _returnvalue 1000.0))
    (set `self.Launched` true)
    (`KismetSystemLibrary.Delay` 0.1)
    (bind _canproceed (`self.CanProceedWithLaunch` (`self.As PLAYER Main Character`)))
    (if _canproceed
      (`self.LaunchCharacter` (* _returnvalue 100000.0))
      (set `self.Launched` false)
      (`PrimitiveComponent.SetSimulatePhysics` (`self.Mesh`) true)
      (set `/Game/Game/PlayerCharacter/Blueprints/MagneticForce.ApplyForce` false (`self.MagneticForce`))
      (`PrimitiveComponent.SetCollisionEnabled` (`self.CapsuleComponent`) "NoCollision")
      (else
        (set `self.Launched` false)))))

(fn `CanProceedWithLaunch`
  (params (actorCollidedWith :type "/Game/Game/PlayerCharacter/Blueprints/PLAYER_MainCharacter Object Reference (by ref)"))
  (returns (canProceed :type Boolean))
  (if (and (`|EnumEquality` (`self.magneticBadDudePolarity`) "NewEnumerator2") (`|EnumEquality` (`/Game/Game/PlayerCharacter/Blueprints/PLAYER_MainCharacter.currentMagneticPolarity` actorCollidedWith) "NewEnumerator1"))
    (return true)
    (elif (and (`|EnumEquality` (`self.magneticBadDudePolarity`) "NewEnumerator1") (`|EnumEquality` (`/Game/Game/PlayerCharacter/Blueprints/PLAYER_MainCharacter.currentMagneticPolarity` actorCollidedWith) "NewEnumerator2"))
      (return true)
      (else
        (return false)))))

(fn `UserConstructionScript`
  (bind _magneticforce (`self.MagneticForce`))
  (set `/Game/Game/PlayerCharacter/Blueprints/MagneticForce.Parent` (`self.CapsuleComponent`) _magneticforce)
  (set `/Game/Game/PlayerCharacter/Blueprints/MagneticForce.Influence` (`self.ColSphere`) _magneticforce)
  (set `/Game/Game/PlayerCharacter/Blueprints/MagneticForce.ApplyForce` true _magneticforce)
  (set `self.Launched` false)
  (if (`self.ActorHasTag` "Positive")
    (`ActorComponent.SetAutoActivate` (`self.positive_fire`) true)
    (set `self.magneticBadDudePolarity` "NewEnumerator1")
    (elif (`self.ActorHasTag` "Negative")
      (`ActorComponent.SetAutoActivate` (`self.negative_fire`) true)
      (set `self.magneticBadDudePolarity` "NewEnumerator2"))))